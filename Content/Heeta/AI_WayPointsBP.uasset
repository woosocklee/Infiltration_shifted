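; AI waypoint path actor that defines a route with a spline and exposes queries on it.
; The construction script aims an arrow at spline key 1 to show the path's direction.
; Functions return the closest spline location or rounded point index for a given position.
; GetWayPonts uses DoN rather than a loop, adding at most one point per call; GetClosestWayPointFromNav is an empty stub loop.
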(fn `GetClosestWayPoint`
  (params (location :type "Vector Structure"))
  (returns (ReturnValue :type "Vector Structure"))
  (return (`SplineComponent.FindLocationClosestToWorldLocation` (`self.Spline`) location "World")))

(fn `GetClosestWayPointFromNav`
  (for _ (`self.GetWayPonts`)
    _))

(fn `GetSplineIndex`
  (params (location :type "Vector Structure"))
  (returns (index :type Integer))
  (return (`KismetMathLibrary.Round` (`SplineComponent.FindInputKeyClosestToWorldLocation` (`self.Spline`) location))))

(fn `GetWayPonts`
  (returns (return :type "Array of Vector Structure"))
  (locals (points :type "Array of Vector Structure"))
  (bind _spline (`self.Spline`))
  (`|ExecutionSequence`
    (:`then_0`
      (bind _counter (`/Engine/EditorBlueprintResources/StandardMacros.Do N` (- (`SplineComponent.GetNumberOfSplinePoints` _spline) 1))
        (:`Exit`
          (`KismetArrayLibrary.Array_Add` (`local.points`) (`SplineComponent.GetLocationAtSplinePoint` _spline _counter "World")))))
    (:`then_1`
      (return (`local.points`)))))

(fn `UserConstructionScript`
  (bind _arrow (`self.Arrow`))
  (`SceneComponent.K2_SetWorldRotation` _arrow (`KismetMathLibrary.FindLookAtRotation` (`SceneComponent.K2_GetComponentLocation` _arrow) (`SplineComponent.GetLocationAtSplineInputKey` (`self.Spline`) 1.0 "World")) false false))